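; LocalPlayerState_BP is a work-in-progress game stopwatch for a mine-disarming game.
; After a short BeginPlay delay, StartTimer runs a looping one-second Delay that increments and prints Time while Counting is true.
; BeginPlay checks NumberDisarmed against the game mode's TotalMinesSpawned only once, right after starting the timer.
; On a match, StopTImer clears Counting, stops Level_Spawner's music and plays a completion sound.
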(event `self.ReceiveBeginPlay`
  (`KismetSystemLibrary.Delay` 4.2)
  ;[1 1 1] Game Stopwatch WIP (astoriea)
  (`self.Start Timer`)
  (bind _asthird_person_game_mode (cast `/Game/ThirdPersonBP/Blueprints/ThirdPersonGameMode` (`GameplayStatics.GetGameMode`)))
  (if (== (`self.Number Disarmed`) (`/Game/ThirdPersonBP/Blueprints/ThirdPersonGameMode.Total Mines Spawned` _asthird_person_game_mode))
    (`self.Stop TImer`)))

(event `Start Timer`
  (bind _time (`self.Time`))
  (set `self.Counting` true)
  (`KismetSystemLibrary.Delay` 1.0 :!label _label)
  (`/Engine/EditorBlueprintResources/StandardMacros.IncrementInt` _time
    (:`  `
      (`KismetSystemLibrary.PrintString` (`KismetStringLibrary.Conv_IntToString` _time) true true (struct :`G` 0.66 :`B` 1.0 :`A` 1.0) 0.1)
      (if (`self.Counting`)
        (goto _label)))))

(event `Stop TImer`
  (set `self.Counting` false)
  (bind _returnvalue (`GameplayStatics.GetActorOfClass` "/Game/Blueprints/Level_Spawner.Level_Spawner_C"))
  (`/Game/Blueprints/Level_Spawner.Stop Music` _returnvalue)
  (`GameplayStatics.PlaySound2D` "/Game/Audio/Complete.Complete" 1.0 1.0 0.0 null null))

(fn `UserConstructionScript`)