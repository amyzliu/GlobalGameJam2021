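; Trap is a beeping proximity bomb that explodes when anything other than a HoveringBot enters its trigger Sphere.
; Detonation spawns an Explosion, calls Exploded on each AnimalWalk inside BlastRadius, destroys the trap and leaves an enlarged ExplosionHoleActor.
; Disarm instead replaces the trap with a Flag.
; An attenuated beep cue starts on BeginPlay and stops when the actor is destroyed.
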(event `/Game/Blueprints/Disarm_Interface.Disarm`
  (`|SpawnActorFromClass` "/Game/Blueprints/Flag.Flag_C" (`KismetMathLibrary.Conv_VectorToTransform` (`self.K2_GetActorLocation`)) "Undefined" "OverrideRootScale" null null)
  (`self.K2_DestroyActor`))

(event `self.Sphere.OnComponentBeginOverlap`
  (params (OverlappedComponent :type "PrimitiveComponent Object Reference") (OtherActor :type "Actor Object Reference") (OtherComp :type "PrimitiveComponent Object Reference") (OtherBodyIndex :type Integer) (bFromSweep :type Boolean) (SweepResult :type "HitResult Structure (by ref)"))
  ;[1 1 1] Explosion
  (`KismetSystemLibrary.PrintString` (`KismetSystemLibrary.GetDisplayName` OtherActor))
  (cast `/Game/ThirdPersonBP/Blueprints/HoveringBot` OtherActor
    (:`CastFailed`
      (`|SpawnActorFromClass` "/Game/Blueprints/Explosion.Explosion_C" (`KismetMathLibrary.MakeTransform` (`self.K2_GetActorLocation`)) "Undefined" "OverrideRootScale" null null)
      (for _array_element (`PrimitiveComponent.GetOverlappingActors` (`self.BlastRadius`) "/Game/Blueprints/AnimalWalk.AnimalWalk_C")
        (bind _asanimal_walk (cast `/Game/Blueprints/AnimalWalk` _array_element))
        (`/Game/Blueprints/AnimalWalk.Exploded` _asanimal_walk))
      (`self.K2_DestroyActor`)
      (`self.OnExploded`))))

(event `OnExploded`
  ;[1 1 1] Spawn Explosion Hole On Explosion Completion
  (`|SpawnActorFromClass` "/Game/Blueprints/ExplosionHoleActor.ExplosionHoleActor_C" (`KismetMathLibrary.MakeTransform` (`self.K2_GetActorLocation`) (struct) (5.0 5.0 5.0)) "Undefined" "OverrideRootScale" null null))

(event `self.ReceiveBeginPlay`
  ;[1 1 1] Beeping Sound Logic
  (bind _returnvalue (`GameplayStatics.SpawnSoundAtLocation` "/Game/Audio/BeepCue.BeepCue" (`self.K2_GetActorLocation`) (struct) 1.0 1.0 0.0 "/Game/Audio/BombDetectionAttenuation.BombDetectionAttenuation" null))
  (set `self.BeepSound` _returnvalue))

(event `self.ReceiveDestroyed`
  ;[1 1 1] Beeping Sound Logic
  (`AudioComponent.Stop` (`self.BeepSound`)))

(fn `UserConstructionScript`)