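; Level spawner actor that sets up a bunny level: score HUD, intro-to-loop music with nature ambience, and random placement of traps, bunnies and carrots.
; Mines and bunnies pick random map locations, retrying a few times to avoid overlapping existing traps; mines and carrots align to the floor normal.
; The spawned mine count goes to ThirdPersonGameMode, and a looping timer keeps dropping single carrots.
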(event `self.ReceiveBeginPlay`
  (`|ExecutionSequence`
    (:`then_0`
      ;[1 1 1] Spawn High Score
      (bind _returnvalue (`|CreateWidget` "/Game/Blueprints/BunnyScoreHUD.BunnyScoreHUD_C"))
      (`UserWidget.AddToViewport` _returnvalue 0)
      (set `self.Bunny HUD Main` _returnvalue))
    (:`then_1`
      (`|ExecutionSequence`
        (:`then_0`
          (`GameplayStatics.SpawnSound2D` "/Game/Audio/Intro_to_Loop.Intro_to_Loop" 1.0 1.0 0.0 null)
          (`KismetSystemLibrary.Delay` 4.1)
          (bind _returnvalue_2 (`GameplayStatics.SpawnSound2D` "/Game/Audio/MusicLoop.MusicLoop" 1.0 1.0 0.0 null))
          (set `self.MySound` _returnvalue_2))
        (:`then_1`
          (`GameplayStatics.PlaySound2D` "/Game/Audio/NatureBirdsCrickets_BW_1500_Cue.NatureBirdsCrickets_BW_1500_Cue" 1.0 1.0 0.0 null null))))
    (:`then_2`
      (`self.Spawn All`))))

(event `Stop Music`
  ;[1 1 1] Pause main theme song
  (`AudioComponent.Stop` (`self.MySound`)))

(event `Spawn All`
  (bind _actors_to_ignore (`self.Actors to Ignore`))
  (bind _width (`self.Width`))
  (bind _number_of_bunnies (`self.Number of Bunnies`))
  (bind _height (`self.Height`))
  (bind _mines_spawned (`self.Spawn Mines` _width _height (`self.Number of Mines`) _actors_to_ignore))
  (`self.Spawn Bunnies` _width _height _number_of_bunnies _actors_to_ignore)
  (`KismetSystemLibrary.K2_SetTimerDelegate` (delegate `Spawn Carrot`) (`self.Carrot Spawn Time`) true)
  (bind _asthird_person_game_mode (cast `/Game/ThirdPersonBP/Blueprints/ThirdPersonGameMode` (`GameplayStatics.GetGameMode`)))
  (set `/Game/ThirdPersonBP/Blueprints/ThirdPersonGameMode.Total Mines Spawned` _mines_spawned _asthird_person_game_mode)
  (set `self.Number Bunnies Spawned` _number_of_bunnies))

(event `Spawn Carrot`
  (`self.Spawn Carrots` (`self.Width`) (`self.Height`) (`KismetMathLibrary.RandomIntegerInRange` 1 1) (`self.Actors to Ignore`)))

(fn `Spawn Bunnies`
  (params (Width :type "Float (double-precision)") (Height :type "Float (double-precision)") (`Number of Bunnies` :type Integer) (ActorsToIgnore :type "Array of Actor Object Reference (by ref)"))
  (locals (NewLocalVar_0 :type "Array of EObjectTypeQuery Enum"))
  (for _ (range 1 (+ `Number of Bunnies` 1))
    (for _ (range 6)
      (bind _location (`/Game/Blueprints/RandomMapLocation.RandomMapLocation` Width Height ActorsToIgnore))
      (bind (_outactors _returnvalue) (`KismetSystemLibrary.SphereOverlapActors` _location 100.0 (`|MakeArray` "ObjectTypeQuery1" "ObjectTypeQuery2" "ObjectTypeQuery4" "ObjectTypeQuery3" :!type "EObjectTypeQuery Enum") "/Game/Blueprints/Trap.Trap_C"))
      (if (not _returnvalue)
        (`|SpawnActorFromClass` "/Game/Blueprints/AnimalWalk.AnimalWalk_C" (`KismetMathLibrary.Conv_VectorToTransform` (+ _location (0.0 0.0 35.0))) "Undefined" "OverrideRootScale" null null)
        (set `self.Number Bunnies Spawned` (+ (`self.Number Bunnies Spawned`) 1))
        (break)))))

(fn `Spawn Carrots`
  (params (Width :type "Float (double-precision)") (Height :type "Float (double-precision)") (`Number of Carrots` :type Integer) (ActorsToIgnore :type "Array of Actor Object Reference (by ref)"))
  (for _ (range 1 (+ `Number of Carrots` 1))
    (bind (_location _normal _normalrotation) (`/Game/Blueprints/RandomMapLocation.RandomMapLocation` Width Height ActorsToIgnore))
    (bind _returnvalue (`|SpawnActorFromClass` "/Game/Blueprints/Carrot.Carrot_C" (`KismetMathLibrary.Conv_VectorToTransform` _location) "Undefined" "OverrideRootScale" null null))
    (if (not (`self.IsActorBeingDestroyed` _returnvalue))
      (`SceneComponent.K2_SetWorldRotation` (`/Game/Blueprints/Carrot.Carrot1` _returnvalue) _normalrotation false false))))

(fn `Spawn Mines`
  (params (Width :type "Float (double-precision)") (Height :type "Float (double-precision)") (`Number of Mines` :type Integer) (ActorsToIgnore :type "Array of Actor Object Reference (by ref)"))
  (returns (`Mines Spawned` :type Integer))
  (locals (SuccessfulMines :type Integer :default 0))
  (set `local.SuccessfulMines` 0)
  (for _ (range 1 (+ `Number of Mines` 1))
    (for _ (range 6)
      (bind (_location _normal _normalrotation) (`/Game/Blueprints/RandomMapLocation.RandomMapLocation` Width Height ActorsToIgnore))
      (bind (_outactors _returnvalue) (`KismetSystemLibrary.SphereOverlapActors` _location 50.0 (`|MakeArray` "ObjectTypeQuery1" "ObjectTypeQuery2" "ObjectTypeQuery4" "ObjectTypeQuery3" :!type "EObjectTypeQuery Enum") "/Game/Blueprints/Trap.Trap_C"))
      (if (not _returnvalue)
        (bind _returnvalue_2 (`|SpawnActorFromClass` "/Game/Blueprints/Trap.Trap_C" (`KismetMathLibrary.Conv_VectorToTransform` _location) "Undefined" "OverrideRootScale" null null))
        (`KismetArrayLibrary.Array_Add` ActorsToIgnore _returnvalue_2)
        (set `/Game/Blueprints/Trap.Floor Rotation` _normalrotation _returnvalue_2)
        (set `local.SuccessfulMines` (+ (`local.SuccessfulMines`) 1))
        (`/Game/Blueprints/Trap.Adjust Rotation` _returnvalue_2)
        (break))))
  (return (`local.SuccessfulMines`)))

(fn `UserConstructionScript`)