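; First-person player character that moves, looks, shows a reticle, and interacts with objects in front of the camera.
; Pressing E traces from the camera and sends an interact message to whatever it hits within close range.
; Every movement or look axis event reruns a similar trace, toggling a disarm prompt widget when a nearby, still-armed Trap is under the crosshair.
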(event `Key|E`
  (params (Key :type "Key Structure"))
  (bind _camera (`self.Camera`))
  (bind _returnvalue (`SceneComponent.K2_GetComponentLocation` _camera))
  ;[1 1 1] Interact
  (:`Pressed`
    (bind (_outhit _returnvalue_2) (`KismetSystemLibrary.LineTraceSingle` _returnvalue (+ _returnvalue (* (`KismetMathLibrary.GetForwardVector` (`SceneComponent.K2_GetComponentRotation` _camera)) 300)) "TraceTypeQuery1"))
    (if _returnvalue_2
      (bind (_bblockinghit _binitialoverlap _time _distance _location _impactpoint _normal _impactnormal _physmat _hitactor) (`GameplayStatics.BreakHitResult` _outhit))
      (`/Engine/EditorBlueprintResources/StandardMacros.CompareFloat` _distance 200.0
        (:`<`
          (message `/Game/Blueprints/Interaction_Interface.Interact` _hitactor))))))

(event `InputAxis|MouseLookHorizontal`
  (params (AxisValue :type "Float (single-precision)"))
  ;[1 1 1] Camera
  (`self.AddControllerYawInput` AxisValue)
  (`self.UpdateDisarmUI` :!label _label))

(event `InputAxis|MouseLookVertical`
  (params (AxisValue :type "Float (single-precision)"))
  ;[1 1 1] Camera
  (`self.AddControllerPitchInput` AxisValue)
  (goto _label))

(event `UpdateDisarmUI`
  (bind _camera (`self.Camera`))
  (bind _disarm_ui (`self.Disarm UI`))
  (bind _showing_disarm_ui (`self.Showing Disarm UI`))
  (bind _returnvalue (`SceneComponent.K2_GetComponentLocation` _camera))
  ;[1 1 1] Update Disarm UI
  (bind (_outhit _returnvalue_2) (`KismetSystemLibrary.LineTraceSingle` _returnvalue (+ _returnvalue (* (`KismetMathLibrary.GetForwardVector` (`SceneComponent.K2_GetComponentRotation` _camera)) 300)) "TraceTypeQuery1"))
  (if _returnvalue_2
    (bind (_bblockinghit _binitialoverlap _time _distance _location _impactpoint _normal _impactnormal _physmat _hitactor) (`GameplayStatics.BreakHitResult` _outhit))
    (bind _astrap (cast `/Game/Blueprints/Trap` _hitactor)
      (:`then`
        (`/Engine/EditorBlueprintResources/StandardMacros.CompareFloat` _distance 200.0
          (:`>`
            (if _showing_disarm_ui :!label _label_2
              (`Widget.RemoveFromParent` _disarm_ui :!label _label_3)
              (set `self.Showing Disarm UI` false)))
          (:`==`
            (goto _label_2))
          (:`<`
            (if _showing_disarm_ui
              (bind _disarmed (`/Game/Blueprints/Trap.Disarmed` _astrap))
              (if _disarmed
                (goto _label_3))
              (elif (not _disarmed)
                (`UserWidget.AddToViewport` _disarm_ui 0)
                (set `self.Showing Disarm UI` true))))))
      (:`CastFailed`
        (goto _label_2)))))

(event `InputAxis|MoveRight`
  (params (AxisValue :type "Float (single-precision)"))
  (bind (_returnvalue_roll _returnvalue_pitch _returnvalue_yaw) (`KismetMathLibrary.BreakRotator` (`self.GetControlRotation`)))
  ;[1 1 1] Movement
  (`self.AddMovementInput` (`KismetMathLibrary.GetRightVector` (`KismetMathLibrary.MakeRotator` 0.0 0.0 _returnvalue_yaw)) AxisValue)
  (`self.UpdateDisarmUI` :!label _label_4))

(event `InputAxis|MoveForward`
  (params (AxisValue :type "Float (single-precision)"))
  (bind (_returnvalue_roll _returnvalue_pitch _returnvalue_yaw) (`KismetMathLibrary.BreakRotator` (`self.GetControlRotation`)))
  ;[1 1 1] Movement
  (`self.AddMovementInput` (`KismetMathLibrary.GetForwardVector` (`KismetMathLibrary.MakeRotator` 0.0 0.0 _returnvalue_yaw)) AxisValue)
  (goto _label_4))

(event `self.ReceiveBeginPlay`
  (bind _returnvalue (`GameplayStatics.GetPlayerController` 0))
  ;[1 1 1] UI
  (bind _returnvalue_2 (`|CreateWidget` "/Game/UI/Recticle.Recticle_C" _returnvalue))
  (`UserWidget.AddToViewport` _returnvalue_2 0)
  (bind _returnvalue_3 (`|CreateWidget` "/Game/UI/Disarm.Disarm_C" _returnvalue))
  (set `self.Disarm UI` _returnvalue_3))

(fn `UserConstructionScript`)