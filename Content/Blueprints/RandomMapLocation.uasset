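; Blueprint helper functions that pick a random navigable ground location on a map and report its surface orientation.
; RandomMapLocation samples the navmesh around the world origin, using the hypotenuse of Width and Height as radius, then passes X and Y to HeightForLocation.
; HeightForLocation traces vertically against WorldStatic objects, skipping ignored actors, and returns hit location, normal and a Z-aligned rotation, without checking for a hit.
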(fn `HeightForLocation`
  (params (X :type "Float (double-precision)") (Y :type "Float (double-precision)") (ActorsToIgnore :type "Array of Actor Object Reference (by ref)"))
  (returns (Location :type "Vector Structure") (Normal :type "Vector Structure") (NormalRotation :type "Rotator Structure"))
  (bind _outhit (`KismetSystemLibrary.LineTraceSingleForObjects` null (`KismetMathLibrary.MakeVector` X Y 50000.0) (`KismetMathLibrary.MakeVector` X Y -50000.0) (`|MakeArray` "ObjectTypeQuery1" :!type "EObjectTypeQuery Enum") false ActorsToIgnore "None" true (struct :`R` 1.0 :`A` 1.0) (struct :`G` 1.0 :`A` 1.0) 100.0))
  (bind (_bblockinghit _binitialoverlap _time _distance _location _impactpoint _normal) (`GameplayStatics.BreakHitResult` _outhit))
  (return _location _normal (`KismetMathLibrary.MakeRotFromZ` _normal)))

(fn `RandomMapLocation`
  (params (Width :type "Float (double-precision)") (Height :type "Float (double-precision)") (ActorsToIgnore :type "Array of Actor Object Reference"))
  (returns (Location :type "Vector Structure") (Normal :type "Vector Structure") (NormalRotation :type "Rotator Structure"))
  (locals (NewLocalVar_0 :type Boolean) (NewLocalVar_1 :type "Array of Actor Object Reference"))
  (bind _randomlocation (`NavigationSystemV1.K2_GetRandomLocationInNavigableRadius` null (`KismetMathLibrary.Vector_Zero`) (`KismetMathLibrary.Hypotenuse` Width Height) null null))
  (bind (_location _normal _normalrotation) (`self.HeightForLocation` (.x _randomlocation) (.y _randomlocation) ActorsToIgnore))
  (return _location _normal _normalrotation))