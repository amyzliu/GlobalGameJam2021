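; Procedural fence actor that builds a terrain-following row of fences along its local X axis in the construction script.
; It fits as many FenceWidth segments as Width allows, spreads leftover space as gaps, and alternates two hierarchical instanced meshes.
; HeightForLocation supplies each segment's ground height and normal, which set its Z offset and tilt along the slope.
; A BlockingPlane is centered and stretched to cover the run.
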(fn `UserConstructionScript`
  (locals (`Fence Width` :type "Float (double-precision)" :default 150.0))
  (bind _blocking_plane (`self.Blocking Plane`))
  (bind _width (`self.Width`))
  (bind _fence_width (`local.Fence Width`))
  (bind _returnvalue (`KismetMathLibrary.FMax` _width _fence_width))
  (bind _returnvalue_2 (`KismetMathLibrary.FTrunc` (/ _returnvalue _fence_width)))
  (bind _returnvalue_3 (- _returnvalue_2 1))
  ;[1 1 1] Blocking Walls
  (`SceneComponent.K2_SetRelativeLocation` _blocking_plane (`KismetMathLibrary.MakeVector` (/ _width 2.0)) false true)
  (`SceneComponent.SetRelativeScale3D` _blocking_plane (`KismetMathLibrary.MakeVector` (/ (+ _width _fence_width) 100.0) 50.0 1.0))
  (for _index (range (+ _returnvalue_3 1))
    (bind _returnvalue_4 (+ (/ _fence_width 2.0) (* _index (+ (/ (- _returnvalue (* _returnvalue_2 _fence_width)) (`KismetMathLibrary.Conv_IntToDouble` _returnvalue_3)) _fence_width))))
    (bind (_returnvalue_location _returnvalue_rotation) (`KismetMathLibrary.BreakTransform` (`KismetMathLibrary.ComposeTransforms` (`KismetMathLibrary.Conv_VectorToTransform` (`KismetMathLibrary.MakeVector` _returnvalue_4)) (`SceneComponent.K2_GetComponentToWorld` (`self.DefaultSceneRoot`)))))
    (bind (_location _normal) (`/Game/Blueprints/RandomMapLocation.HeightForLocation` (.x _returnvalue_location) (.y _returnvalue_location) (`|MakeArray`)))
    (bind _returnvalue_5 (`KismetMathLibrary.GreaterGreater_VectorRotator` _normal (`KismetMathLibrary.NegateRotator` _returnvalue_rotation)))
    (`InstancedStaticMeshComponent.AddInstance` (select `int` (mod _index 2) :`0` (`self.HierarchicalInstancedStaticMesh1`) :`1` (`self.HierarchicalInstancedStaticMesh2`)) (`KismetMathLibrary.MakeTransform` (`KismetMathLibrary.MakeVector` _returnvalue_4 0.0 (- (.z _location) (.z _returnvalue_location))) (`KismetMathLibrary.ComposeRotators` (`KismetMathLibrary.RotatorFromAxisAndAngle` (0.0 0.0 1.0) 90.0) (`KismetMathLibrary.RotatorFromAxisAndAngle` (`KismetMathLibrary.MakeVector` 0.0 (`KismetMathLibrary.SignOfFloat` (`KismetMathLibrary.VSize` (`KismetMathLibrary.ProjectVectorOnToVector` _returnvalue_5 (1.0 0.0 0.0))))) (`KismetMathLibrary.DegAtan2` (.x (`KismetMathLibrary.Normal` _returnvalue_5)) (.z (`KismetMathLibrary.Normal` _returnvalue_5)))))))))